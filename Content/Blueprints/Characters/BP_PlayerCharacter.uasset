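; Player character Blueprint that relays the player's actions to animations and effects on the W_Game HUD widget.
; On BeginPlay it caches the widget from MainGameMode and starts its UI flicker.
; The PlayerFire event triggers the widget's fire UI, while Tick polls movement velocity and starts the walk animation whenever the player moves and that animation is not already playing.
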(event `self.PlayerFire`
  (params (DamageGiven :type "Float (single-precision)"))
  (bind _widgetgame (`self.WidgetGame`))
  (`/Engine/EditorBlueprintResources/StandardMacros.IsValid` _widgetgame
    (:`Is Valid`
      (`/Game/Blueprints/Widget/W_Game.FireUI` _widgetgame))))

(event `self.ReceiveBeginPlay`
  (bind _asmain_game_mode (cast `/Game/Blueprints/MainGameMode` (`GameplayStatics.GetGameMode`)))
  (bind _asw_game (cast `/Game/Blueprints/Widget/W_Game` (`/Game/Blueprints/MainGameMode.GameWidget` _asmain_game_mode)))
  (bind _output_get (set `self.WidgetGame` _asw_game))
  (`/Game/Blueprints/Widget/W_Game.BeginFlickerUI` _output_get))

(event `self.ReceiveTick`
  (params (DeltaSeconds :type "Float (single-precision)"))
  (bind _widgetgame (`self.WidgetGame`))
  (if (and (> (`KismetMathLibrary.VSize` (`MovementComponent.Velocity` (`self.MovementComp`))) 0.0) (not (`UserWidget.IsAnimationPlaying` _widgetgame (`/Game/Blueprints/Widget/W_Game.Walking` _widgetgame))))
    (`/Game/Blueprints/Widget/W_Game.WalkAnim` (`self.WidgetGame`))))

(fn `UserConstructionScript`)