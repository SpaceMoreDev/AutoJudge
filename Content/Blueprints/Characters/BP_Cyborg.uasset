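; BP_Cyborg is an enemy character that chases the player and dies from any damage a player controller instigates.
; StartAI, which nothing in this Blueprint calls, re-issues AIMoveTo toward the first player pawn on a short repeating delay.
; On player damage, it turns to face the player, plays a death montage and destroys itself shortly after, with no health check.
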(event `self.StartAI`
  (`|AIMoveTo` self (0.0 0.0 0.0) (`GameplayStatics.GetPlayerPawn` 0) :!label _label
    (:`then`
      (`KismetSystemLibrary.Delay` 0.2)
      (goto _label))))

(event `self.ReceiveAnyDamage`
  (params (Damage :type "Float (single-precision)") (DamageType :type "DamageType Object Reference") (InstigatedBy :type "Controller Object Reference") (DamageCauser :type "Actor Object Reference"))
  (if (`Controller.IsPlayerController` InstigatedBy)
    (`self.K2_SetActorRotation` (`KismetMathLibrary.FindLookAtRotation` (`self.K2_GetActorLocation`) (`self.K2_GetActorLocation` (`GameplayStatics.GetPlayerPawn` 0))))
    (`self.PlayAnimMontage` "/Game/Art/3D/Cyborg/animations/Death_Montage.Death_Montage")
    (`KismetSystemLibrary.Delay` 0.3)
    (`self.K2_DestroyActor`)))

(fn `UserConstructionScript`)