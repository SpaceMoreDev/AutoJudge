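; Player character Blueprint that handles gun and HUD feedback, health, score access and look sensitivity.
; BeginPlay applies the Game Instance's sensitivity and caches the game widget from MainGameMode.
; Tick sways the HUD, score and health widgets against look input using FInterpTo.
; Firing triggers widget feedback and a brief gun kickback, while damage plays a hit animation and calls GameOver when health drops below one.
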(event `self.PlayerFire`
  (params (DamageGiven :type "Float (single-precision)"))
  (bind _widget_game (`self.Widget Game`))
  (`/Engine/EditorBlueprintResources/StandardMacros.IsValid` _widget_game
    (:`Is Valid`
      (`/Game/Blueprints/Widget/W_Game.FireUI` _widget_game)
      (`SceneComponent.K2_AddRelativeLocation` (`self.Gun`) (-5.0 0.0 0.0) false false)
      (`KismetSystemLibrary.Delay` 0.1)
      (`SceneComponent.K2_SetRelativeLocation` (`self.Gun`) (`self.gun original loc`) false false))))

(event `self.ReceiveBeginPlay`
  (bind _asgame_instance_main (cast `/Game/Blueprints/Widget/GameInstance_Main` (`GameplayStatics.GetGameInstance`)))
  (`self.SetSens` (`/Game/Blueprints/Widget/GameInstance_Main.Sensitivity` _asgame_instance_main))
  (bind _asmain_game_mode (cast `/Game/Blueprints/MainGameMode` (`GameplayStatics.GetGameMode`)))
  (bind _asw_game (cast `/Game/Blueprints/Widget/W_Game` (`/Game/Blueprints/MainGameMode.GameWidget` _asmain_game_mode)))
  (bind _output_get (set `self.Widget Game` _asw_game))
  (`/Game/Blueprints/Widget/W_Game.BeginFlickerUI` _output_get)
  (set `self.gun original loc` (`SceneComponent.RelativeLocation` (`self.Gun`))))

(event `self.ReceiveTick`
  (params (DeltaSeconds :type "Float (single-precision)"))
  (bind (_returnvalue_x _returnvalue_y) (`KismetMathLibrary.BreakVector2D` (`|GetInputActionValue`)))
  (bind _widget_game (`self.Widget Game`))
  (bind _uimove_amount (`self.UIMove Amount`))
  (bind _returnvalue (`WidgetLayoutLibrary.SlotAsCanvasSlot` (`/Game/Blueprints/Widget/W_Game.HUD` _widget_game)))
  (bind _returnvalue_2 (`WidgetLayoutLibrary.SlotAsCanvasSlot` (`/Game/Blueprints/Widget/W_Game.Score` _widget_game)))
  (bind _returnvalue_3 (`WidgetLayoutLibrary.SlotAsCanvasSlot` (`/Game/Blueprints/Widget/W_Game.Health` _widget_game)))
  (bind (_returnvalue_x_2 _returnvalue_y_2) (`KismetMathLibrary.BreakVector2D` (`CanvasPanelSlot.GetPosition` _returnvalue)))
  (bind (_returnvalue_x_3 _returnvalue_y_3) (`KismetMathLibrary.BreakVector2D` (`CanvasPanelSlot.GetPosition` _returnvalue_2)))
  (bind (_returnvalue_x_4 _returnvalue_y_4) (`KismetMathLibrary.BreakVector2D` (`CanvasPanelSlot.GetPosition` _returnvalue_3)))
  (bind (_x _y) (`self.Interp Position` _returnvalue_x_2 _returnvalue_y_2 _returnvalue_x _returnvalue_y _uimove_amount))
  (bind (_x_2 _y_2) (`self.Interp Position` _returnvalue_x_3 _returnvalue_y_3 _returnvalue_x _returnvalue_y _uimove_amount))
  (bind (_x_3 _y_3) (`self.Interp Position` _returnvalue_x_4 _returnvalue_y_4 _returnvalue_x _returnvalue_y (`self.UIMove Amount`)))
  (`/Engine/EditorBlueprintResources/StandardMacros.IsValid` _widget_game
    (:`Is Valid`
      (`CanvasPanelSlot.SetPosition` _returnvalue (`KismetMathLibrary.MakeVector2D` _x _y))
      (`CanvasPanelSlot.SetPosition` _returnvalue_2 (`KismetMathLibrary.MakeVector2D` _x_2 _y_2))
      (`CanvasPanelSlot.SetPosition` _returnvalue_3 (`KismetMathLibrary.MakeVector2D` _x_3 _y_3)))))

(event `self.ReceiveAnyDamage`
  (params (Damage :type "Float (single-precision)") (DamageType :type "DamageType Object Reference") (InstigatedBy :type "Controller Object Reference") (DamageCauser :type "Actor Object Reference"))
  (bind _widget_game (`self.Widget Game`))
  (`/Engine/EditorBlueprintResources/StandardMacros.IsValid` _widget_game
    (:`Is Valid`
      (`/Game/Blueprints/Widget/W_Game.BeginHitAnim` _widget_game)
      (if (< (`HealthComponent.Health` (`self.Health`)) 1.0)
        (bind _asmain_game_mode (cast `/Game/Blueprints/MainGameMode` (`GameplayStatics.GetGameMode`)))
        (`/Game/Blueprints/MainGameMode.GameOver` _asmain_game_mode)))))

(fn `AddHealth`
  (params (`new health` :type "Float (double-precision)"))
  (bind _health (`self.Health`))
  (set `HealthComponent.Health` (+ (`HealthComponent.Health` _health) `new health`) _health))

(fn `GetHealth`
  (returns (Health :type "Float (single-precision)"))
  (return (`HealthComponent.Health` (`self.Health`))))

(fn `GetScore`
  (returns (`Score Counter` :type Integer))
  (return (`self.ScoreCounter`)))

(fn `Interp Position`
  (params (Current_X :type "Float (double-precision)") (Current_Y :type "Float (double-precision)") (X_Axis :type "Float (double-precision)") (Y_Axis :type "Float (double-precision)") (Amount :type "Float (double-precision)" :default 20.0))
  (returns (X :type "Float (double-precision)") (Y :type "Float (double-precision)"))
  (bind _returnvalue (`GameplayStatics.GetWorldDeltaSeconds`))
  (return (`KismetMathLibrary.FInterpTo` Current_X (* (* X_Axis Amount) -1.0) _returnvalue 5.0) (`KismetMathLibrary.FInterpTo` Current_Y (* Y_Axis Amount) _returnvalue 5.0)))

(fn `SetSens`
  (params (sens :type "Float (double-precision)"))
  (set `self.LookSpeed` (* sens 100.0)))

(fn `UserConstructionScript`)